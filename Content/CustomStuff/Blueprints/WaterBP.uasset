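; Water volume that floats and slows overlapping physics objects and toggles the player's underwater state, refilling jumps on exit.
; Overlapping actors are tracked in an array, and each Tick pushes their root primitive upward using its BuoyancyComponent value or a default.
; An opposing drag force is added above a velocity threshold.
; The construction script gives the Boundaries mesh a dynamic water material with U/V parameters scaled to its size.
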(event `self.ReceiveTick`
  (params (DeltaSeconds :type "Float (single-precision)"))
  (for _array_element (`self.Array of Overlaps`)
    (`self.Actor Under Water` _array_element)))

(event `self.ReceiveActorBeginOverlap`
  (params (OtherActor :type "Actor Object Reference"))
  (`KismetArrayLibrary.Array_AddUnique` (`self.Array of Overlaps`) OtherActor)
  (bind _asplayer_bp (cast `/Game/CustomStuff/Blueprints/PlayerBP` OtherActor))
  (`/Game/CustomStuff/Blueprints/PlayerBP.GoUnderwater` _asplayer_bp))

(event `self.ReceiveActorEndOverlap`
  (params (OtherActor :type "Actor Object Reference"))
  (`KismetArrayLibrary.Array_RemoveItem` (`self.Array of Overlaps`) OtherActor)
  (bind _asplayer_bp (cast `/Game/CustomStuff/Blueprints/PlayerBP` OtherActor))
  (`/Game/CustomStuff/Blueprints/PlayerBP.GoOverwater` _asplayer_bp)
  (set `/Game/CustomStuff/Blueprints/PlayerBP.Jumps Left` (`/Game/CustomStuff/Blueprints/PlayerBP.Max Jumps` _asplayer_bp) _asplayer_bp))

(event `Actor Under Water`
  (params (Actor :type "Actor Object Reference"))
  (bind _returnvalue (`self.GetComponentByClass` Actor "/Game/CustomStuff/Blueprints/BuoyancyComponent.BuoyancyComponent_C"))
  (bind _asprimitive_component (cast `PrimitiveComponent` (`Actor.RootComponent` Actor)))
  (bind _returnvalue_2 (`SceneComponent.GetComponentVelocity` _asprimitive_component))
  (`PrimitiveComponent.AddForce` _asprimitive_component (+ (* (* (0.0 0.0 1.0) (`KismetMathLibrary.SelectFloat` (`/Game/CustomStuff/Blueprints/BuoyancyComponent.Buoyancy` _returnvalue) (`self.Default Buoyancy`) (`KismetSystemLibrary.IsValid` _returnvalue))) (`self.Water Strength`)) (select `bool` (> (`KismetMathLibrary.VSize` _returnvalue_2) (`self.Drag Velocity`)) :`true` (* (`KismetMathLibrary.NegateVector` _returnvalue_2) (`self.Drag Strength`)))) "None" false))

(fn `UserConstructionScript`
  (bind _boundaries (`self.Boundaries`))
  (bind _returnvalue (`KismetMaterialLibrary.CreateDynamicMaterialInstance` "/Game/CustomStuff/Materials/M_Translucent_Water_Lake.M_Translucent_Water_Lake"))
  (`PrimitiveComponent.SetMaterial` _boundaries 0 _returnvalue)
  (`MaterialInstanceDynamic.SetScalarParameterValue` _returnvalue "U" (.x (* (`SceneComponent.K2_GetComponentScale` _boundaries) 0.5)))
  (`MaterialInstanceDynamic.SetScalarParameterValue` _returnvalue "V" (.y (* (`SceneComponent.K2_GetComponentScale` _boundaries) 0.5))))