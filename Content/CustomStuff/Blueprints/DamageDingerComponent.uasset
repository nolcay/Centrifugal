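; An actor component that shows floating damage numbers above its owner whenever it takes damage.
; On BeginPlay it binds to the owner's OnTakeAnyDamage; unless the OwnerDead flag is set, each hit spawns a BillboardTextBP at a configurable height.
; The text shows the negated damage with configurable color and size, and the actor is destroyed after a Lifetime delay.
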(event `self.ReceiveBeginPlay`
  (add `Actor.OnTakeAnyDamage` (`self.GetOwner`) (delegate `Damage`)))

(event `Damage`
  (params (DamagedActor :type "Actor Object Reference") (Damage :type "Float (double-precision)") (DamageType :type "DamageType Object Reference") (InstigatedBy :type "Controller Object Reference") (DamageCauser :type "Actor Object Reference"))
  (if (not (`self.Owner Dead?`))
    (bind _returnvalue (`|SpawnActorFromClass` "/Game/CustomStuff/Blueprints/BillboardTextBP.BillboardTextBP_C" (`KismetMathLibrary.MakeTransform` (`KismetMathLibrary.MakeVector` (.x (`Actor.K2_GetActorLocation` (`self.GetOwner`))) (.y (`Actor.K2_GetActorLocation` (`self.GetOwner`))) (+ (.z (`Actor.K2_GetActorLocation` (`self.GetOwner`))) (`self.Height`))) (struct)) "Undefined" "OverrideRootScale" null null))
    (bind _textrender (`TextRenderActor.TextRender` _returnvalue))
    (`TextRenderComponent.K2_SetText` _textrender (`KismetTextLibrary.Conv_StringToText` (`KismetStringLibrary.Concat_StrStr` "-" (`KismetStringLibrary.Conv_DoubleToString` Damage))))
    (`TextRenderComponent.SetTextRenderColor` _textrender (`KismetMathLibrary.Conv_LinearColorToColor` (`self.Color`)))
    (`TextRenderComponent.SetWorldSize` _textrender (`self.Text Size`))
    (`KismetSystemLibrary.Delay` (`self.Lifetime`))
    (`Actor.K2_DestroyActor` _returnvalue)))