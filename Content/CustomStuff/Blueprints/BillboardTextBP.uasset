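; BillboardTextBP is a world text actor that turns to face each player's camera separately.
; On BeginPlay it spawns a centered text actor copy per PlayerController, owned by that controller's pawn and visible only to its owner.
; Tick rotates each copy toward its mapped camera and mirrors the source TextRender's color, font, text and size onto all copies.
; The copies are destroyed along with the billboard.
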(event `self.ReceiveDestroyed`
  (for _array_element (`self.TextRenders`)
    (`self.K2_DestroyActor` (`ActorComponent.GetOwner` _array_element))))

(event `self.ReceiveBeginPlay`
  (bind _outactors (`GameplayStatics.GetAllActorsOfClass` "/Script/Engine.PlayerController"))
  (for _array_element _outactors
    (bind _returnvalue (`|SpawnActorFromClass` (`self.Text Class`) (`self.GetTransform`) "Undefined" "OverrideRootScale"))
    (`BlueprintMapLibrary.Map_Add` (`self.Positions`) (`PlayerController.PlayerCameraManager` _array_element) _returnvalue)
    (bind _textrender (`TextRenderActor.TextRender` _returnvalue))
    (`TextRenderComponent.SetHorizontalAlignment` _textrender "EHTA_Center")
    (`self.SetOwner` _returnvalue (`Controller.K2_GetPawn` _array_element))
    (`PrimitiveComponent.SetOnlyOwnerSee` _textrender true)
    (`KismetArrayLibrary.Array_Add` (`self.TextRenders`) _textrender)))

(event `self.ReceiveTick`
  (params (DeltaSeconds :type "Float (single-precision)"))
  (bind _textrender (`self.TextRender`))
  (bind _positions (`self.Positions`))
  (bind _keys (`BlueprintMapLibrary.Map_Keys` _positions))
  (for _array_element _keys
    (bind _textrender_2 (`TextRenderActor.TextRender` (`BlueprintMapLibrary.Map_Find` _positions _array_element)))
    (`SceneComponent.K2_SetWorldRotation` _textrender_2 (`KismetMathLibrary.FindLookAtRotation` (`SceneComponent.K2_GetComponentLocation` _textrender_2) (`PlayerCameraManager.GetCameraLocation` _array_element)) false false)
    (for _array_element_2 (`self.TextRenders`)
      (`TextRenderComponent.SetTextRenderColor` _array_element_2 (`TextRenderComponent.TextRenderColor` _textrender))
      (`TextRenderComponent.SetFont` _array_element_2 (`TextRenderComponent.Font` _textrender))
      (`TextRenderComponent.K2_SetText` _array_element_2 (`TextRenderComponent.Text` _textrender))
      (`TextRenderComponent.SetWorldSize` _array_element_2 (`KismetMathLibrary.VSize` (`TextRenderComponent.GetTextWorldSize` _textrender))))))

(fn `UserConstructionScript`)