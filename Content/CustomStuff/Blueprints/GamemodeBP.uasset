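; Game mode for a two-player local game that spawns, possesses and sets up each player's PlayerBP and HUD at tagged PlayerStarts.
; It routes movement, jump and float input to both pawns, with toggled gates switching P2 between input sets including gamepad.
; Tick polls health for explosion and delayed respawn, and moves each spawn point to that player's latest activated checkpoint.
; A finish counter prints the victor after two finishes.
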(event `Start Game`
  (bind _outactors (`GameplayStatics.GetAllActorsOfClass` "/Script/Engine.PlayerStart"))
  (`GameplayStatics.CreatePlayer` -1)
  (`|ExecutionSequence`
    (:`then_0`
      (bind _outactors_2 (`GameplayStatics.GetAllActorsOfClass` "/Script/Engine.PlayerController"))
      (for _array_element _outactors_2
        (bind _returnvalue (`GameplayStatics.GetPlayerControllerID` _array_element))
        (switch `int` _returnvalue
          (:`0`
            (for _array_element_2 _outactors
              (if (== (`PlayerStart.PlayerStartTag` _array_element_2) "P1")
                (break)))
            (bind _output_get (set `self.P1 Spawn Transform` (`self.GetTransform` _array_element_2)))
            (bind _returnvalue_2 (`|CreateWidget` "/Game/CustomStuff/UI/HUD_P1.HUD_P1_C" _array_element))
            (`UserWidget.AddToPlayerScreen` _returnvalue_2 0)
            (`self.Spawn Player` _array_element _output_get))
          (:`1`
            (for _array_element_3 _outactors
              (if (== (`PlayerStart.PlayerStartTag` _array_element_3) "P2")
                (break)))
            (bind _output_get_2 (set `self.P2 Spawn Transform` (`self.GetTransform` _array_element_3)))
            (bind _returnvalue_3 (`|CreateWidget` "/Game/CustomStuff/UI/HUD_P2.HUD_P2_C" _array_element))
            (`UserWidget.AddToPlayerScreen` _returnvalue_3 0)
            (`self.Spawn Player` _array_element _output_get_2)))))
    (:`then_1`
      (bind _outactors_3 (`GameplayStatics.GetAllActorsOfClass` "/Game/CustomStuff/Blueprints/CheckpointBP.CheckpointBP_C"))
      (for _array_element_4 _outactors_3
        (switch `int` (`/Game/CustomStuff/Blueprints/CheckpointBP.Player ID` _array_element_4)
          (:`0`
            (`KismetArrayLibrary.Array_Add` (`self.Checkpoints P1`) _array_element_4))
          (:`1`
            (`KismetArrayLibrary.Array_Add` (`self.Checkpoints P2`) _array_element_4)))))))

(event `Spawn Player`
  (params (`Player Controller` :type "PlayerController Object Reference") (Transform :type "Transform Structure"))
  (`self.K2_DestroyActor` (`Controller.K2_GetPawn` `Player Controller`))
  (bind _returnvalue (`|SpawnActorFromClass` "/Game/CustomStuff/Blueprints/PlayerBP.PlayerBP_C" Transform "Undefined" "OverrideRootScale" null null))
  (`Controller.Possess` `Player Controller` _returnvalue))

(event `InputAxis|Move P1`
  (params (AxisValue :type "Float (single-precision)"))
  (if (not (`self.P1 Dead?`))
    (`/Game/CustomStuff/Blueprints/PlayerBP.Move` (`self.P1`) AxisValue)))

(event `self.ReceiveBeginPlay`
  (bind _returnvalue (`GameplayStatics.GetPlayerController` 1))
  (bind _returnvalue_2 (`GameplayStatics.GetPlayerController` 0))
  (`|ExecutionSequence`
    (:`then_0`
      (`self.Start Game`))
    (:`then_1`
      (bind _outactors (`GameplayStatics.GetAllActorsOfClass` "/Script/Engine.PlayerController"))
      (for _array_element _outactors
        (bind _asplayer_bp (cast `/Game/CustomStuff/Blueprints/PlayerBP` (`Controller.K2_GetPawn` _array_element)))
        (`PlayerController.SetViewTargetWithBlend` _array_element _asplayer_bp 0.0 "VTBlend_Linear" 0.0 false)))
    (:`then_2`
      (bind _asplayer_bp_2 (cast `/Game/CustomStuff/Blueprints/PlayerBP` (`Controller.K2_GetPawn` _returnvalue_2)))
      (bind _output_get (set `self.P1` _asplayer_bp_2))
      (`self.EnableInput` _returnvalue_2)
      (`PrimitiveComponent.SetMaterial` (`/Game/CustomStuff/Blueprints/PlayerBP.Sphere` _output_get) 0 "/Game/CustomStuff/Materials/P1Mat.P1Mat"))
    (:`then_3`
      (bind _asplayer_bp_3 (cast `/Game/CustomStuff/Blueprints/PlayerBP` (`Controller.K2_GetPawn` _returnvalue)))
      (bind _output_get_2 (set `self.P2` _asplayer_bp_3))
      (`self.EnableInput` _returnvalue)
      (`PrimitiveComponent.SetMaterial` (`/Game/CustomStuff/Blueprints/PlayerBP.Sphere` _output_get_2) 0 "/Game/CustomStuff/Materials/P2Mat.P2Mat"))
    (:`then_4`
      (`GameplayStatics.SpawnSound2D` "/Game/CustomStuff/Sounds/345851__hargissssound__spring-birds-raw-new-jersey.345851__hargissssound__spring-birds-raw-new-jersey" 0.75))))

(event `InputAction|Jump P1`
  (params (Key :type "Key Structure"))
  (bind _p1 (`self.P1`))
  (:`Pressed`
    (if (`self.P1 Dead?`)
      _
      (elif (not (or (`/Game/CustomStuff/Blueprints/PlayerBP.Is Under Water?` _p1) (not (`PrimitiveComponent.IsGravityEnabled` (`/Game/CustomStuff/Blueprints/PlayerBP.Sphere` _p1)))))
        (`/Game/CustomStuff/Blueprints/PlayerBP.Jump` _p1)))))

(event `InputAxis|Float P1`
  (params (AxisValue :type "Float (single-precision)"))
  (bind _p1 (`self.P1`))
  (if (`self.P1 Dead?`)
    _
    (elif (or (`/Game/CustomStuff/Blueprints/PlayerBP.Is Under Water?` _p1) (not (`PrimitiveComponent.IsGravityEnabled` (`/Game/CustomStuff/Blueprints/PlayerBP.Sphere` _p1))))
      (`/Game/CustomStuff/Blueprints/PlayerBP.Float` _p1 AxisValue))))

(event `InputAxis|Move P2`
  (params (AxisValue :type "Float (single-precision)"))
  (`/Engine/EditorBlueprintResources/StandardMacros.Gate` false :!label _label
    (:`Exit`
      (if (not (`self.P2 Dead?`))
        (`/Game/CustomStuff/Blueprints/PlayerBP.Move` (`self.P2`) AxisValue)))))

(event `InputAction|Jump P2`
  (params (Key :type "Key Structure"))
  (bind _p2 (`self.P2`))
  (:`Pressed`
    (`/Engine/EditorBlueprintResources/StandardMacros.Gate` false :!label _label_2
      (:`Exit`
        (if (`self.P2 Dead?`)
          _
          (elif (not (or (`/Game/CustomStuff/Blueprints/PlayerBP.Is Under Water?` _p2) (not (`PrimitiveComponent.IsGravityEnabled` (`/Game/CustomStuff/Blueprints/PlayerBP.Sphere` _p2)))))
            (`/Game/CustomStuff/Blueprints/PlayerBP.Jump` _p2)))))))

(event `InputAxis|Float P2`
  (params (AxisValue :type "Float (single-precision)"))
  (bind _p2 (`self.P2`))
  (`/Engine/EditorBlueprintResources/StandardMacros.Gate` false :!label _label_3
    (:`Exit`
      (if (`self.P2 Dead?`)
        _
        (elif (or (`/Game/CustomStuff/Blueprints/PlayerBP.Is Under Water?` _p2) (not (`PrimitiveComponent.IsGravityEnabled` (`/Game/CustomStuff/Blueprints/PlayerBP.Sphere` _p2))))
          (`/Game/CustomStuff/Blueprints/PlayerBP.Float` _p2 AxisValue))))))

(event `InputAction|P2 Activate Controller`
  (params (Key :type "Key Structure"))
  (bind _p2 (`self.P2`))
  (bind _p2_dead_ (`self.P2 Dead?`))
  (bind _returnvalue (`PrimitiveComponent.IsGravityEnabled` (`/Game/CustomStuff/Blueprints/PlayerBP.Sphere` _p2)))
  (:`Pressed`
    (`|ExecutionSequence`
      (:`then_0`
        (goto _label :!via `Toggle`))
      (:`then_1`
        (goto _label_2 :!via `Toggle`))
      (:`then_2`
        (goto _label_3 :!via `Toggle`))
      (:`then_3`
        (goto _label_4 :!via `Toggle`))
      (:`then_4`
        (goto _label_5 :!via `Toggle`))
      (:`then_5`
        (goto _label_6 :!via `Toggle`)))))

(event `InputAxis|Move P2 Gamepad`
  (params (AxisValue :type "Float (single-precision)"))
  (`/Engine/EditorBlueprintResources/StandardMacros.Gate` true :!label _label_4
    (:`Exit`
      (if (not (`self.P2 Dead?`))
        (`/Game/CustomStuff/Blueprints/PlayerBP.Move` (`self.P2`) AxisValue)))))

(event `InputAction|Jump P2 Gamepad`
  (params (Key :type "Key Structure"))
  (bind _p2 (`self.P2`))
  (:`Pressed`
    (`/Engine/EditorBlueprintResources/StandardMacros.Gate` true :!label _label_5
      (:`Exit`
        (if (`self.P2 Dead?`)
          _
          (elif (`PrimitiveComponent.IsGravityEnabled` (`/Game/CustomStuff/Blueprints/PlayerBP.Sphere` _p2))
            (`/Game/CustomStuff/Blueprints/PlayerBP.Jump` _p2)))))))

(event `InputAxis|Float P2 Gamepad`
  (params (AxisValue :type "Float (single-precision)"))
  (bind _p2 (`self.P2`))
  (`/Engine/EditorBlueprintResources/StandardMacros.Gate` true :!label _label_6
    (:`Exit`
      (if (`self.P2 Dead?`)
        _
        (elif (not (`PrimitiveComponent.IsGravityEnabled` (`/Game/CustomStuff/Blueprints/PlayerBP.Sphere` _p2)))
          (`/Game/CustomStuff/Blueprints/PlayerBP.Float` _p2 AxisValue))))))

(event `Finished`
  (params (Player :type "/Game/CustomStuff/Blueprints/PlayerEnum Enum" :default "NewEnumerator0"))
  (bind _numoffinishes (`self.NumOfFinishes`))
  (`/Engine/EditorBlueprintResources/StandardMacros.IncrementInt` _numoffinishes
    (:`  `
      (if (== _numoffinishes 2)
        (`KismetSystemLibrary.Delay` 2.0)
        (`KismetSystemLibrary.PrintString` (`KismetStringLibrary.Concat_StrStr` "Game Finished! Victor: " (`|GetEnumeratorNameAsString` (cast `/Game/CustomStuff/Blueprints/PlayerEnum` (- 0 Player)))))))))

(event `self.ReceiveTick`
  (params (DeltaSeconds :type "Float (single-precision)"))
  (`|ExecutionSequence`
    (:`then_0`
      (if (and (<= (`/Game/CustomStuff/Blueprints/PlayerBP.Health` (`self.P1`)) 0.0) (not (`self.P1 Dead?`)))
        (set `self.P1 Dead?` true)
        (`SceneComponent.SetVisibility` (`/Game/CustomStuff/Blueprints/PlayerBP.Sphere` (`self.P1`)) false false)
        (`GameplayStatics.SpawnEmitterAtLocation` "/Game/CustomStuff/ParticleEffects/Explosion.Explosion" (`SceneComponent.K2_GetComponentLocation` (`/Game/CustomStuff/Blueprints/PlayerBP.Sphere` (`self.P1`))))
        (set `/Game/CustomStuff/Blueprints/DamageDingerComponent.Owner Dead?` true (`/Game/CustomStuff/Blueprints/PlayerBP.DamageDingerComponent` (`self.P1`)))
        (`KismetSystemLibrary.Delay` (`self.Respawn Time`))
        (`self.K2_SetActorTransform` (`self.P1`) (`self.P1 Spawn Transform`) false false)
        (`SceneComponent.SetVisibility` (`/Game/CustomStuff/Blueprints/PlayerBP.Sphere` (`self.P1`)) true false)
        (set `self.P1 Dead?` false)
        (set `/Game/CustomStuff/Blueprints/PlayerBP.Health` (`/Game/CustomStuff/Blueprints/PlayerBP.Base Health` (`self.P1`)) (`self.P1`))
        (set `/Game/CustomStuff/Blueprints/DamageDingerComponent.Owner Dead?` false (`/Game/CustomStuff/Blueprints/PlayerBP.DamageDingerComponent` (`self.P1`)))))
    (:`then_1`
      (if (and (<= (`/Game/CustomStuff/Blueprints/PlayerBP.Health` (`self.P2`)) 0.0) (not (`self.P2 Dead?`)))
        (set `self.P2 Dead?` true)
        (`SceneComponent.SetVisibility` (`/Game/CustomStuff/Blueprints/PlayerBP.Sphere` (`self.P2`)) false false)
        (`GameplayStatics.SpawnEmitterAtLocation` "/Game/CustomStuff/ParticleEffects/Explosion.Explosion" (`SceneComponent.K2_GetComponentLocation` (`/Game/CustomStuff/Blueprints/PlayerBP.Sphere` (`self.P2`))))
        (set `/Game/CustomStuff/Blueprints/DamageDingerComponent.Owner Dead?` true (`/Game/CustomStuff/Blueprints/PlayerBP.DamageDingerComponent` (`self.P2`)))
        (`KismetSystemLibrary.Delay` (`self.Respawn Time`))
        (`self.K2_SetActorTransform` (`self.P2`) (`self.P2 Spawn Transform`) false false)
        (`SceneComponent.SetVisibility` (`/Game/CustomStuff/Blueprints/PlayerBP.Sphere` (`self.P2`)) true false)
        (set `self.P2 Dead?` false)
        (set `/Game/CustomStuff/Blueprints/PlayerBP.Health` (`/Game/CustomStuff/Blueprints/PlayerBP.Base Health` (`self.P2`)) (`self.P2`))
        (set `/Game/CustomStuff/Blueprints/DamageDingerComponent.Owner Dead?` false (`/Game/CustomStuff/Blueprints/PlayerBP.DamageDingerComponent` (`self.P2`)))))
    (:`then_2`
      (for _array_element (`self.Checkpoints P1`)
        (if (`/Game/CustomStuff/Blueprints/CheckpointBP.Activation State` _array_element)
          (if (!= _array_element (`self.Active CP P1`))
            (bind _output_get (set `self.Active CP P1` _array_element))
            (set `self.P1 Spawn Transform` (`self.GetTransform` _output_get))
            (for _array_element_2 (`self.Checkpoints P1`)
              (if (!= _array_element_2 _output_get)
                (`/Game/CustomStuff/Blueprints/CheckpointBP.Deactivated` _array_element_2)))))))
    (:`then_3`
      (for _array_element_3 (`self.Checkpoints P2`)
        (if (`/Game/CustomStuff/Blueprints/CheckpointBP.Activation State` _array_element_3)
          (if (!= _array_element_3 (`self.Active CP P2`))
            (bind _output_get_2 (set `self.Active CP P2` _array_element_3))
            (set `self.P2 Spawn Transform` (`self.GetTransform` _output_get_2))
            (for _array_element_4 (`self.Checkpoints P2`)
              (if (!= _array_element_4 _output_get_2)
                (`/Game/CustomStuff/Blueprints/CheckpointBP.Deactivated` _array_element_4)))))))))

(fn `CP Verify Player`
  (params (Actor :type "Actor Object Reference") (`Player ID` :type Integer))
  (returns (`Is correct player?` :type Boolean))
  (bind _asplayer_bp (cast `/Game/CustomStuff/Blueprints/PlayerBP` Actor)
    (:`then`
      (switch `int` `Player ID`
        (:`Default`
          _)
        (:`0`
          (return (== (`self.P1`) _asplayer_bp)))
        (:`1`
          (return (== (`self.P2`) _asplayer_bp)))))
    (:`CastFailed`
      _))
  (return false))

(fn `UserConstructionScript`)