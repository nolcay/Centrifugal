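; Two-player cone actor with a Box trigger that marks players dead and a Finish trigger that reports a finish to GamemodeBP.
; Box identifies P1 or P2, sets its dead flag, blends that player's camera to this actor and sets the root's constraint mode to None.
; Finish calls Finished with one enum value for P1 and the other for any other overlapping actor, without checking for P2.
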(event `self.Box.OnComponentBeginOverlap`
  (params (OverlappedComponent :type "PrimitiveComponent Object Reference") (OtherActor :type "Actor Object Reference") (OtherComp :type "PrimitiveComponent Object Reference") (OtherBodyIndex :type Integer) (bFromSweep :type Boolean) (SweepResult :type "HitResult Structure (by ref)"))
  (bind _blend_time (`self.Blend Time`))
  (bind _asplayer_bp (cast `/Game/CustomStuff/Blueprints/PlayerBP` OtherActor))
  (bind _asgamemode_bp (cast `/Game/CustomStuff/Blueprints/GamemodeBP` (`GameplayStatics.GetGameMode`)))
  (bind _p1 (`/Game/CustomStuff/Blueprints/GamemodeBP.P1` _asgamemode_bp))
  (if (== _p1 _asplayer_bp)
    (set `/Game/CustomStuff/Blueprints/GamemodeBP.P1 Dead?` true _asgamemode_bp)
    (bind _asplayer_controller (cast `PlayerController` (`Pawn.GetController` _p1)))
    (`PlayerController.SetViewTargetWithBlend` _asplayer_controller self _blend_time "VTBlend_Cubic" 0.0 true)
    (bind _asprimitive_component (cast `PrimitiveComponent` (`Actor.RootComponent` _p1)))
    (`PrimitiveComponent.SetConstraintMode` _asprimitive_component "None")
    (else
      (bind _p2 (`/Game/CustomStuff/Blueprints/GamemodeBP.P2` _asgamemode_bp))
      (if (== _p2 _asplayer_bp)
        (set `/Game/CustomStuff/Blueprints/GamemodeBP.P2 Dead?` true _asgamemode_bp)
        (bind _asplayer_controller_2 (cast `PlayerController` (`Pawn.GetController` _p2)))
        (`PlayerController.SetViewTargetWithBlend` _asplayer_controller_2 self _blend_time "VTBlend_Cubic" 0.0 true)
        (bind _asprimitive_component_2 (cast `PrimitiveComponent` (`Actor.RootComponent` _p2)))
        (`PrimitiveComponent.SetConstraintMode` _asprimitive_component_2 "None")))))

(event `self.Finish.OnComponentBeginOverlap`
  (params (OverlappedComponent :type "PrimitiveComponent Object Reference") (OtherActor :type "Actor Object Reference") (OtherComp :type "PrimitiveComponent Object Reference") (OtherBodyIndex :type Integer) (bFromSweep :type Boolean) (SweepResult :type "HitResult Structure (by ref)"))
  (bind _asgamemode_bp (cast `/Game/CustomStuff/Blueprints/GamemodeBP` (`GameplayStatics.GetGameMode`)))
  (if (== OtherActor (`/Game/CustomStuff/Blueprints/GamemodeBP.P1` _asgamemode_bp))
    (`/Game/CustomStuff/Blueprints/GamemodeBP.Finished` _asgamemode_bp "NewEnumerator0")
    (else
      (`/Game/CustomStuff/Blueprints/GamemodeBP.Finished` _asgamemode_bp "NewEnumerator1"))))

(fn `UserConstructionScript`)