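; Extra jump pickup that temporarily raises the overlapping PlayerBP's MaxJumps, clamped to a configurable maximum.
; On overlap it caches the old jump limit, hides its sphere, closes a gate against repeat pickups and plays a power-up sound.
; Separate delays restore the cached limit with a power-down sound after the duration, and show the sphere and reopen the gate after the respawn time.
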(event `self.ReceiveActorBeginOverlap`
  (params (OtherActor :type "Actor Object Reference"))
  (`/Engine/EditorBlueprintResources/StandardMacros.Gate` false :!label _label
    (:`Exit`
      (bind _asplayer_bp (cast `/Game/CustomStuff/Blueprints/PlayerBP` OtherActor))
      (bind _max_jumps (`/Game/CustomStuff/Blueprints/PlayerBP.Max Jumps` _asplayer_bp))
      (set `self.Old Jump Value` _max_jumps)
      (set `/Game/CustomStuff/Blueprints/PlayerBP.Max Jumps` (`KismetMathLibrary.Clamp` (+ _max_jumps (`self.Increment Max Jumps`)) 0 (`self.Max Value of Max Jumps`)) _asplayer_bp)
      (`SceneComponent.SetVisibility` (`self.Sphere`) false true)
      (`|ExecutionSequence`
        (:`then_0`
          (goto _label :!via `Close`))
        (:`then_1`
          (`KismetSystemLibrary.Delay` (`self.Duration in Seconds`))
          (set `/Game/CustomStuff/Blueprints/PlayerBP.Max Jumps` (`self.Old Jump Value`) _asplayer_bp)
          (bind _returnvalue (`self.K2_GetActorLocation` _asplayer_bp))
          (`GameplayStatics.PlaySoundAtLocation` "/Game/CustomStuff/Sounds/138490__randomationpictures__powerdown-2.138490__randomationpictures__powerdown-2" _returnvalue))
        (:`then_2`
          (`GameplayStatics.PlaySoundAtLocation` "/Game/CustomStuff/Sounds/368651_josepharaoh99_game-powerup.368651_josepharaoh99_game-powerup" _returnvalue)
          (`KismetSystemLibrary.Delay` (`self.Respawn in Seconds`))
          (`SceneComponent.SetVisibility` (`self.Sphere`) true true)
          (goto _label :!via `Open`))))))

(fn `UserConstructionScript`)