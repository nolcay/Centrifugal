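; Metallic powerup pickup that temporarily makes the overlapping PlayerBP less buoyant and gives it a metallic physical material.
; A player tag prevents stacking, and a gate blocks further pickups while the sphere is hidden until respawn.
; Parallel delays run from pickup: one restores the player's buoyancy, material and tag with a power-down sound, the other reshows the sphere and reopens the gate.
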(event `self.ReceiveActorBeginOverlap`
  (params (OtherActor :type "Actor Object Reference"))
  (bind _powerup_tag (`self.Powerup Tag`))
  (bind _asplayer_bp (cast `/Game/CustomStuff/Blueprints/PlayerBP` OtherActor))
  (bind _tags (`Actor.Tags` _asplayer_bp))
  (if (== (`KismetArrayLibrary.Array_Find` _tags _powerup_tag) -1)
    (`/Engine/EditorBlueprintResources/StandardMacros.Gate` false :!label _label
      (:`Exit`
        (`KismetArrayLibrary.Array_Add` _tags _powerup_tag)
        (bind _buoyancycomponent (`/Game/CustomStuff/Blueprints/PlayerBP.BuoyancyComponent` _asplayer_bp))
        (bind _buoyancy (`/Game/CustomStuff/Blueprints/BuoyancyComponent.Buoyancy` _buoyancycomponent))
        (set `self.Old Buoyancy` _buoyancy)
        (set `/Game/CustomStuff/Blueprints/BuoyancyComponent.Buoyancy` (- _buoyancy (`self.Buoyancy Decrement`)) _buoyancycomponent)
        (bind _asprimitive_component (cast `PrimitiveComponent` (`Actor.RootComponent` _asplayer_bp)))
        (`PrimitiveComponent.SetPhysMaterialOverride` _asprimitive_component "/Game/CustomStuff/PhysMats/Player_Metallic.Player_Metallic")
        (`SceneComponent.SetVisibility` (`self.Sphere`) false true)
        (`|ExecutionSequence`
          (:`then_0`
            (goto _label :!via `Close`))
          (:`then_1`
            (`KismetSystemLibrary.Delay` (`self.Duration in Seconds`))
            (set `/Game/CustomStuff/Blueprints/BuoyancyComponent.Buoyancy` (`self.Old Buoyancy`) _buoyancycomponent)
            (bind _returnvalue (`self.K2_GetActorLocation` _asplayer_bp))
            (`GameplayStatics.PlaySoundAtLocation` "/Game/CustomStuff/Sounds/138490__randomationpictures__powerdown-2.138490__randomationpictures__powerdown-2" _returnvalue)
            (`KismetArrayLibrary.Array_RemoveItem` (`Actor.Tags` _asplayer_bp) (`self.Powerup Tag`))
            (`PrimitiveComponent.SetPhysMaterialOverride` _asprimitive_component "/Game/CustomStuff/PhysMats/Player.Player"))
          (:`then_2`
            (`GameplayStatics.PlaySoundAtLocation` "/Game/CustomStuff/Sounds/368651_josepharaoh99_game-powerup.368651_josepharaoh99_game-powerup" _returnvalue)
            (`KismetSystemLibrary.Delay` (`self.Respawn in Seconds`))
            (`SceneComponent.SetVisibility` (`self.Sphere`) true true)
            (goto _label :!via `Open`)))))))

(fn `UserConstructionScript`)