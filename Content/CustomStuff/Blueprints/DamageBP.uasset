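; DamageBP is an actor that turns the actor it is attached to into an environmental hazard that damages whatever it hits.
; On BeginPlay it plays a quiet ambient sound and binds to the parent's OnActorHit, printing a warning if no valid parent exists.
; Each hit applies environmental damage with the parent as causer, then plays a hit sound at the parent's location after a short delay.
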(event `self.ReceiveBeginPlay`
  (bind _returnvalue (`self.GetAttachParentActor`))
  (`GameplayStatics.SpawnSoundAtLocation` (`self.Ambient Sound`) (`self.K2_GetActorLocation`) (struct) 0.1)
  (`/Engine/EditorBlueprintResources/StandardMacros.IsValid` _returnvalue
    (:`Is Valid`
      (add `self.OnActorHit` _returnvalue (delegate `Hit`)))
    (:`Is Not Valid`
      (`KismetSystemLibrary.PrintString` "Invalid Parent Actor"))))

(event `Hit` :!signature `self.OnActorHit`
  (params (SelfActor :type "Actor Object Reference") (OtherActor :type "Actor Object Reference") (NormalImpulse :type "Vector Structure") (Hit :type "HitResult Structure (by ref)"))
  (bind _returnvalue (`self.GetAttachParentActor`))
  (`GameplayStatics.ApplyDamage` OtherActor (`self.Damage`) null _returnvalue "/Engine/EngineDamageTypes/DmgTypeBP_Environmental.DmgTypeBP_Environmental_C")
  (`KismetSystemLibrary.Delay` 0.2)
  (`GameplayStatics.SpawnSoundAtLocation` (`self.Hit Sound`) (`self.K2_GetActorLocation` _returnvalue) (struct) 2.0))

(fn `UserConstructionScript`)