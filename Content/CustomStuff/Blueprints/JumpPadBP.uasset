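; Jump pad that launches actors that hit it by overriding their root primitive component's physics velocity.
; The launch vector follows the Arrow component's world rotation, with strength scaled by its world X scale.
; The AbsMax helper picks the larger-magnitude value per axis between current and launch velocity, so faster existing motion on any axis is kept, even if it opposes the launch.
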(event `self.ReceiveHit`
  (params (MyComp :type "PrimitiveComponent Object Reference") (Other :type "Actor Object Reference") (OtherComp :type "PrimitiveComponent Object Reference") (bSelfMoved :type Boolean) (HitLocation :type "Vector Structure") (HitNormal :type "Vector Structure") (NormalImpulse :type "Vector Structure") (Hit :type "HitResult Structure (by ref)"))
  (bind _arrow (`self.Arrow`))
  (bind _asprimitive_component (cast `PrimitiveComponent` (`Actor.RootComponent` Other)))
  (bind _returnvalue (`PrimitiveComponent.GetPhysicsLinearVelocity` _asprimitive_component "None"))
  (`PrimitiveComponent.SetPhysicsLinearVelocity` _asprimitive_component (`KismetMathLibrary.MakeVector` (`self.AbsMax` (.x _returnvalue) (.x (`KismetMathLibrary.GreaterGreater_VectorRotator` (* (1000.0 0.0 0.0) (.x (`SceneComponent.K2_GetComponentScale` _arrow))) (`SceneComponent.K2_GetComponentRotation` _arrow)))) (`self.AbsMax` (.y _returnvalue) (.y (`KismetMathLibrary.GreaterGreater_VectorRotator` (* (1000.0 0.0 0.0) (.x (`SceneComponent.K2_GetComponentScale` _arrow))) (`SceneComponent.K2_GetComponentRotation` _arrow)))) (`self.AbsMax` (.z _returnvalue) (.z (`KismetMathLibrary.GreaterGreater_VectorRotator` (* (1000.0 0.0 0.0) (.x (`SceneComponent.K2_GetComponentScale` _arrow))) (`SceneComponent.K2_GetComponentRotation` _arrow))))) false "None"))

(fn `UserConstructionScript`)