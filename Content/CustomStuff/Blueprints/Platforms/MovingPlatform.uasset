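; Moving platform actor that travels along a Track spline by time, optionally taking roll, pitch and yaw from the spline.
; Each tick advances the clamped platform time by direction and places the platform at constant velocity; with StopOnHit, a swept hit rolls the time back.
; At endpoints it stops, ping-pongs with an optional wait, or restarts from the opposite end.
; The construction script applies start direction, time and track duration to preview placement.
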(event `self.ReceiveTick`
  (params (DeltaSeconds :type "Float (single-precision)"))
  (set `self.DeltaTime` DeltaSeconds)
  (if (`self.bMovePlatform`)
    (`|ExecutionSequence`
      (:`then_0`
        ;[1 1 1] Platform Movement
        (`self.UpdatePlatformTime`)
        (`self.SetPlatformLocationAndRotation` (`self.bStopOnHit`)))
      (:`then_1`
        (bind _return (`self.EndpointReached`))
        (if _return
          (if (`self.bLoop`)
            (switch `/Game/CustomStuff/Blueprints/Platforms/PlatformMovement` (`self.PlatformMovement`)
              (:`NewEnumerator0`
                (`self.PingPongEvent`))
              (:`NewEnumerator1`
                (`self.LoopFromBeginningEvent`)))
            (else
              (set `self.bMovePlatform` false))))))))

(event `PingPongEvent`
  ;[1 1 1] Change Movement Direction
  (set `self.PlatformDirection` (* (`self.PlatformDirection`) -1))
  ;[1 1 1] Endpoint Delay
  (if (`self.bWaitAtEndpoints`)
    (set `self.bMovePlatform` false)
    (`KismetSystemLibrary.Delay` (`self.PlatformEndpointWaitTime`))
    (`self.UpdatePlatformTime`)
    (`self.SetPlatformLocationAndRotation` (`self.bStopOnHit`))
    (set `self.bMovePlatform` true)))

(event `LoopFromBeginningEvent`
  (if (> (`self.PlatformDirection`) 0)
    (set `self.PlatformTime` 0.0)
    (else
      (set `self.PlatformTime` (`SplineComponent.Duration` (`self.Track`))))))

(fn `EndpointReached`
  (returns (return :type Boolean))
  (locals (bEndpointReached :type Boolean))
  (`|ExecutionSequence`
    (:`then_0`
      (`/Engine/EditorBlueprintResources/StandardMacros.CompareInt` (`self.PlatformDirection`)
        (:`>`
          (set `local.bEndpointReached` (`KismetMathLibrary.NearlyEqual_FloatFloat` (`self.PlatformTime`) (`SplineComponent.Duration` (`self.Track`)))))
        (:`==`
          (`KismetSystemLibrary.PrintString` "*** Platform Direction equals 0 ***" false))
        (:`<`
          (set `local.bEndpointReached` (`KismetMathLibrary.NearlyEqual_FloatFloat` (`self.PlatformTime`))))))
    (:`then_1`
      (return (`local.bEndpointReached`)))))

(fn `SetPlatformLocationAndRotation`
  (params (Sweep :type Boolean))
  (locals (lSweep :type Boolean) (NewRotation :type "Rotator Structure"))
  (bind (_returnvalue_roll _returnvalue_pitch _returnvalue_yaw) (`KismetMathLibrary.BreakRotator` (`SplineComponent.GetRotationAtTime` (`self.Track`) (`self.PlatformTime`) "World" true)))
  (bind (_returnvalue_roll_2 _returnvalue_pitch_2 _returnvalue_yaw_2) (`KismetMathLibrary.BreakRotator` (`SceneComponent.K2_GetComponentRotation` (`self.MovingPlatform`))))
  (set `local.lSweep` Sweep)
  (set `local.NewRotation` (`KismetMathLibrary.MakeRotator` (`KismetMathLibrary.SelectFloat` _returnvalue_roll _returnvalue_roll_2 (`self.bUseTrack'sRoll`)) (`KismetMathLibrary.SelectFloat` _returnvalue_pitch _returnvalue_pitch_2 (`self.bUseTrack'sPitch`)) (`KismetMathLibrary.SelectFloat` _returnvalue_yaw _returnvalue_yaw_2 (`self.bUseTrack'sYaw`))))
  (bind _sweephitresult (`SceneComponent.K2_SetWorldLocationAndRotation` (`self.MovingPlatform`) (`SplineComponent.GetLocationAtTime` (`self.Track`) (`self.PlatformTime`) "World" true) (`local.NewRotation`) (`local.lSweep`) false))
  (bind (_bblockinghit _binitialoverlap) (`GameplayStatics.BreakHitResult` _sweephitresult))
  (if (or _bblockinghit _binitialoverlap)
    (set `self.PlatformTime` (`self.cachedPlatformTime`))))

(fn `UpdatePlatformTime`
  (set `self.cachedPlatformTime` (`self.PlatformTime`))
  (set `self.PlatformTime` (`KismetMathLibrary.FClamp` (+ (* (`self.PlatformDirection`) (`self.DeltaTime`)) (`self.PlatformTime`)) 0.0 (`SplineComponent.Duration` (`self.Track`))))
  (return))

(fn `UserConstructionScript`
  (set `self.PlatformDirection` (`self.PlatformStartDirection`))
  (set `SplineComponent.Duration` (`self.TrackDuration`) (`self.Track`))
  (set `self.PlatformTime` (`self.PlatformStartTime`))
  (`self.SetPlatformLocationAndRotation` false))