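; Checkpoint actor that activates when a player verified for its PlayerID overlaps it.
; On overlap, an inactive checkpoint asks GamemodeBP's CPVerifyPlayer to validate the overlapping actor before activating.
; Activation swaps the Trigger material, calls Activated for listeners and sets ActivationState to block retriggering.
; Deactivated restores the inactive material and clears that state; the construction script applies the same material initially.
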(event `self.ReceiveActorBeginOverlap`
  (params (OtherActor :type "Actor Object Reference"))
  (if (not (`self.Activation State`))
    (bind _asgamemode_bp (cast `/Game/CustomStuff/Blueprints/GamemodeBP` (`GameplayStatics.GetGameMode`)))
    (bind _is_correct_player_ (`/Game/CustomStuff/Blueprints/GamemodeBP.CP Verify Player` _asgamemode_bp OtherActor (`self.Player ID`)))
    (if _is_correct_player_
      (`self.Activated`))))

(event `Activated`
  (`PrimitiveComponent.SetMaterial` (`self.Trigger`) 0 (`self.Activated Material`))
  (`self.Activated!`)
  (set `self.Activation State` true))

(event `Deactivated`
  (`PrimitiveComponent.SetMaterial` (`self.Trigger`) 0 (`self.Deactivated Material`))
  (set `self.Activation State` false))

(fn `UserConstructionScript`
  (`PrimitiveComponent.SetMaterial` (`self.Trigger`) 0 (`self.Deactivated Material`)))